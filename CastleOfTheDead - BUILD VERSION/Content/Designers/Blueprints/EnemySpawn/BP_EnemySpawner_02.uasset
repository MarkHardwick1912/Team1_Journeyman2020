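; Enemy spawner actor that places up to two EnemyAi actors at random navigable points close to its root.
; BeginPlay runs a Delay-based loop that spawns at a fixed interval while CanSpawn is set and polls more often while it is off.
; AllowSpawn and RemoveSpwan toggle that flag.
; On reaching the cap, the loop clears the flag and ends for good.
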(event Custom|AllowSpawn
  (Variables|Default|SetCanSpawn true))

(event Custom|RemoveSpwan
  (Variables|Default|SetCanSpawn false))

(event EventBeginPlay
  (if (Variables|Default|GetCanSpawn) :!label _label
    (if (== (Variables|Default|GetSpawnCount) 2.0)
      (Variables|Default|SetCanSpawn false)
      (else
        (Variables|Default|SetSpawnCount (+ (Variables|Default|GetSpawnCount) 1.0))
        (Game|SpawnActorfromClass "/Game/Designers/AI/EnemyAi.EnemyAi_C" (Math|Transform|MakeTransform (.RandomLocation (Class|NavigationSystemV1|GetRandomPointinNavigableRadius (Transformation|GetWorldLocation (Variables|Default|GetDefaultSceneRoot)) 1e+02 0 0)) "0, 0, 0" "1,1,1") "Undefined" 0 0)
        (Utilities|FlowControl|Delay 2.0)
        (goto _label)))
    (else
      (Utilities|FlowControl|Delay 0.2)
      (goto _label))))

(fn ConstructionScript)