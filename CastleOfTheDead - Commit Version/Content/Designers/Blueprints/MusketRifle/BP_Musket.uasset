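; VR musket actor that BP_MotionController picks up and drops, with optional two-handed aiming and gun-mounted hand meshes replacing the controller hands.
; Tick rotates the gun toward the second hand and toggles ammo/reload displays.
; Fire input from the holding hand spends ammo, line-traces, applies damage, updates game-mode score and spawns effects.
; Timelines drive a material parameter for disintegrate/reintegrate; hit-bone damage logic is disconnected.
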(event OnComponentBeginOverlap(SecondHandTrigger)
  (params (OverlappedComponent :type Primitive%20Component%20Object%20Reference) (OtherActor :type Actor%20Object%20Reference) (OtherComp :type Primitive%20Component%20Object%20Reference) (OtherBodyIndex :type Integer) (bFromSweep :type Boolean) (SweepResult :type Hit%20Result%20Structure%20%28by%20ref%29))
  (bind _firsthand (Variables|Default|GetFirstHand))
  (bind _returnvalue (Components|GetOwner _firsthand))
  (bind _asbp_motion_controller (Utilities|Casting|CastToBP_MotionController _returnvalue))
  (bind _hand (Variables|/Game/VirtualRealityBP/Blueprints/BP_MotionController.BP_MotionController_C|GetHand _asbp_motion_controller))
  ;[1 1 1] Picking Up With Second Hand
  (if (Variables|Default|GetbIsFirstHandAttached)
    (bind _asbp_motion_controller_2 (Utilities|Casting|CastToBP_MotionController OtherActor))
    (if (not (Actor|ActorHasTag (Variables|/Game/VirtualRealityBP/Blueprints/BP_MotionController.BP_MotionController_C|GetAttachedActor _asbp_motion_controller_2) "HeldObject"))
      (if (and (Utilities|Enum|Equal(Enum) (Variables|/Game/VirtualRealityBP/Blueprints/BP_MotionController.BP_MotionController_C|GetGripState _asbp_motion_controller_2) "NewEnumerator2") (!= (Variables|/Game/VirtualRealityBP/Blueprints/BP_MotionController.BP_MotionController_C|GetMotionController _asbp_motion_controller_2) _firsthand))
        (Variables|Default|SetbIsSecondHandTrackingActive true)
        (bind _output_get (Variables|Default|SetSecondHand (Variables|/Game/VirtualRealityBP/Blueprints/BP_MotionController.BP_MotionController_C|GetMotionController _asbp_motion_controller_2)))
        (Rendering|SetVisibility _output_get false false)
        (if (Utilities|Enum|Equal(Enum) _hand "Left")
          (Rendering|SetVisibility (Variables|Default|GetHandBL) true false)
          (elif (Utilities|Enum|Equal(Enum) _hand "Right")
            (Rendering|SetVisibility (Variables|Default|GetHandFL) true false)))))))

(event OnComponentEndOverlap(SecondHandTrigger)
  (params (OverlappedComponent :type Primitive%20Component%20Object%20Reference) (OtherActor :type Actor%20Object%20Reference) (OtherComp :type Primitive%20Component%20Object%20Reference) (OtherBodyIndex :type Integer))
  ;[1 1 1] Dropping Second hand
  (if (Variables|Default|GetbIsSecondHandTrackingActive)
    (Utilities|IsValid (Variables|Default|GetSecondHand)
      (:Is%20Valid
        (if (and (.bSuccess (Utilities|Casting|CastToBP_MotionController (Components|GetOwner (Variables|Default|GetSecondHand)))) (Utilities|Enum|NotEqual(Enum) (Variables|/Game/VirtualRealityBP/Blueprints/BP_MotionController.BP_MotionController_C|GetGripState (.AsBP%20Motion%20Controller (Utilities|Casting|CastToBP_MotionController (Components|GetOwner (Variables|Default|GetSecondHand))))) "NewEnumerator2"))
          (Variables|Default|SetbIsSecondHandTrackingActive false :!label _label)
          (Rendering|SetVisibility (Variables|/Game/VirtualRealityBP/Blueprints/BP_MotionController.BP_MotionController_C|GetHandMesh (stale OnComponentBeginOverlap(SecondHandTrigger) _asbp_motion_controller_2)) true false)
          (Variables|Default|SetSecondHand 0)
          (Transformation|SetRelativeRotation (Variables|Debug|GetStaticMeshComponent) (Variables|Default|GetOneHandRotation) false true)
          (Rendering|SetVisibility (Variables|Default|GetHandFL) false false)))
      (:Is%20Not%20Valid
        (goto _label)))))

(event Custom|Disintegrate
  ;[1 1 1] Disintegration
  (Components|Activation|Activate (Variables|Default|GetGun_Disintegration) false)
  (bind _returnvalue (Rendering|Material|CreateDynamicMaterialInstance (Variables|Debug|GetStaticMeshComponent) 0 0 "None" :!class /Script/Engine.PrimitiveComponent))
  (bind _isa (Utilities|FlowControl|FlipFlop)
    (:A
      (bind _newtrack_0 (Timeline|Timeline_0 Play)
        (:Update
          (Rendering|Material|SetScalarParameterValue _returnvalue "Amount" _newtrack_0 :!class /Script/Engine.MaterialInstanceDynamic)
          (if _isa
            (Utilities|FlowControl|Delay 0.5)
            (Components|Activation|Activate (Variables|Default|GetGun_Reintegration) false)
            (CallFunction|Disintegrate)))))
    (:B
      (Timeline|Timeline_0 Reverse))))

(event Custom|Reintegrate
  ;[1 1 1] Disintegration
  (bind _returnvalue (Rendering|Material|CreateDynamicMaterialInstance (Variables|Debug|GetStaticMeshComponent) 0 0 "None" :!class /Script/Engine.PrimitiveComponent))
  (bind _newtrack_0 (Timeline|Timeline_1 PlayFromStart)
    (:Update
      (Rendering|Material|SetScalarParameterValue _returnvalue "Amount" _newtrack_0 :!class /Script/Engine.MaterialInstanceDynamic))))

(event EventPickup
  (params (AttachTo :type Scene%20Component%20Object%20Reference))
  ;[1 1 1] Picking Up Gun
  (if (not (Variables|Default|GetbGrabSwordHandle))
    (if (not (Variables|Default|GetbIsFirstHandAttached))
      (Physics|SetSimulatePhysics (Variables|Debug|GetStaticMeshComponent) false)
      (Transformation|AttachComponentToComponent (VehicleSound|GetRootComponent) AttachTo "None" "SnapToTarget" "SnapToTarget" "KeepWorld" false)
      (Transformation|SetRelativeLocationAndRotation (Variables|Debug|GetStaticMeshComponent) "3.030000,-2.380000,1.570000" (Variables|Default|GetOneHandRotation) false true)
      (Variables|Default|SetbIsFirstHandAttached true)
      (Variables|Default|SetbIsSecondHandTrackingActive false)
      (Variables|Default|SetFirstHand AttachTo)
      (Input|EnableInput (Game|GetPlayerController 0))
      (if (Utilities|Enum|Equal(Enum) (Variables|/Game/VirtualRealityBP/Blueprints/BP_MotionController.BP_MotionController_C|GetHand (.AsBP%20Motion%20Controller (Utilities|Casting|CastToBP_MotionController (Components|GetOwner (Variables|Default|GetFirstHand))))) "Right")
        (Rendering|SetVisibility (Variables|/Game/VirtualRealityBP/Blueprints/BP_MotionController.BP_MotionController_C|GetHandMesh (.AsBP%20Motion%20Controller (Utilities|Casting|CastToBP_MotionController (Components|GetOwner (Variables|Default|GetFirstHand))))) false false)
        (Rendering|SetVisibility (Variables|Default|GetHandBR) true false)
        (elif (Utilities|Enum|Equal(Enum) (Variables|/Game/VirtualRealityBP/Blueprints/BP_MotionController.BP_MotionController_C|GetHand (.AsBP%20Motion%20Controller (Utilities|Casting|CastToBP_MotionController (Components|GetOwner (Variables|Default|GetFirstHand))))) "Left")
          (Rendering|SetVisibility (Variables|/Game/VirtualRealityBP/Blueprints/BP_MotionController.BP_MotionController_C|GetHandMesh (.AsBP%20Motion%20Controller (Utilities|Casting|CastToBP_MotionController (Components|GetOwner (Variables|Default|GetFirstHand))))) false false)
          (Rendering|SetVisibility (Variables|Default|GetHandBL) true false))))))

(event EventTick
  (params (DeltaSeconds :type Float%20%28single-precision%29))
  (bind _secondhand (Variables|Default|GetSecondHand))
  (bind _firsthand (Variables|Default|GetFirstHand))
  (bind _returnvalue (Transformation|GetWorldLocation _firsthand))
  (bind _returnvalue_2 (Transformation|GetWorldLocation _secondhand))
  (bind _returnvalue_3 (Math|Rotator|FindLookatRotation _returnvalue _returnvalue_2))
  (bind (_roll _pitch _yaw) (Math|Rotator|BreakRotator _returnvalue_3))
  ;[1 1 1] 2 handed tracking
  (Utilities|FlowControl|Sequence
    (:then_0
      (if (and (Variables|Default|GetbIsSecondHandTrackingActive) (Utilities|IsValid (Variables|Default|GetSecondHand)))
        (Transformation|SetWorldRotation (Variables|Debug|GetStaticMeshComponent) (Math|Rotator|CombineRotators (Variables|Default|GetOneHandRotation) (Math|Rotator|MakeRotator (.Roll (Math|Rotator|BreakRotator (Transformation|GetWorldRotation _firsthand))) _pitch _yaw)) false false)))
    (:then_1
      ;[1 1 1] Ammo Counter/Reload UI
      (if (<= (Variables|Default|GetAmmo) 0.0)
        (Rendering|SetVisibility (Variables|Default|GetReload) true false)
        (Rendering|SetVisibility (Variables|Default|GetAmmoCounter) false false)
        (else
          (Rendering|SetVisibility (Variables|Default|GetReload) false false)
          (Rendering|SetVisibility (Variables|Default|GetAmmoCounter) true false))))))

(event EventDrop
  ;[1 1 1] Dropping gun
  (Physics|SetSimulatePhysics (Variables|Debug|GetStaticMeshComponent) true)
  (Transformation|DetachFromActor "KeepWorld" "KeepWorld" "KeepWorld")
  (Variables|Default|SetbIsFirstHandAttached false)
  (Variables|Default|SetbIsSecondHandTrackingActive false)
  (Input|DisableInput (Game|GetPlayerController 0) 0)
  (Rendering|SetVisibility (Variables|Default|GetHandFL) false false)
  (Rendering|SetVisibility (Variables|/Game/VirtualRealityBP/Blueprints/BP_MotionController.BP_MotionController_C|GetHandMesh (.AsBP%20Motion%20Controller (Utilities|Casting|CastToBP_MotionController (Components|GetOwner (Variables|Default|GetFirstHand))))) true false))

(event Input|ActionEvents|InputActionFireRight
  (params (Key :type Key%20Structure))
  (bind _arrow (Variables|Default|GetArrow))
  (bind _arrow_muzzleflash (Variables|Default|GetArrow_Muzzleflash))
  (bind _basedamage (Variables|Default|GetBaseDamage))
  (bind _returnvalue (Transformation|GetWorldLocation _arrow))
  ;[1 1 1] Check if Firing in Correct Hand and fire line trace
  (:Pressed
    (if (Utilities|Enum|Equal(Enum) (Variables|/Game/VirtualRealityBP/Blueprints/BP_MotionController.BP_MotionController_C|GetHand (.AsBP%20Motion%20Controller (Utilities|Casting|CastToBP_MotionController (Components|GetOwner (Variables|Default|GetFirstHand))))) "Right")
      (if (Variables|Default|GetCan%20Fire)
        (if (<= (Variables|Default|GetAmmo) 0.0)
          (Audio|PlaySound2D "/Game/Designers/Audio/vo_reload_16.vo_reload_16" 1.0 1.0 0.0 0 0)
          (else
            (Variables|Default|SetAmmo (- (Variables|Default|GetAmmo) 1.0))
            (Variables|Default|SetCan%20Fire false)
            (Audio|PlaySound2D "/Game/Designers/Audio/Musket_Single_Shot_Close_03.Musket_Single_Shot_Close_03" 1.0 1.0 0.0 0 0)
            (bind _returnvalue_2 (Effects|SpawnEmitteratLocation "/Game/InfinityBladeEffects/Effects/FX_Monsters/FX_Monster_Chicken/P_ChickenMaster_MuzzleFlash_01.P_ChickenMaster_MuzzleFlash_01" (Transformation|GetWorldLocation _arrow_muzzleflash) (Transformation|GetWorldRotation _arrow_muzzleflash)))
            (Transformation|SetWorldScale3D _returnvalue_2 "0.200000,0.200000,0.200000")
            (bind _outhit (Collision|LineTraceByChannel _returnvalue (+ _returnvalue (* (Math|Vector|GetForwardVector _arrow) 5e+03)) "TraceTypeQuery2" false 0 "None"))
            (Utilities|FlowControl|Delay 0.35)
            (Variables|Default|SetCan%20Fire true)
            (bind _astime_power_up (Utilities|Casting|CastToTime_Power_Up (.HitActor (Collision|BreakHitResult _outhit)))
              (:then
                (Game|Damage|ApplyDamage _astime_power_up _basedamage 0 0))
              (:CastFailed
                (bind _ashealth_power_up (Utilities|Casting|CastToHealth_Power_Up (.HitActor (Collision|BreakHitResult _outhit)))
                  (:then
                    (Game|Damage|ApplyDamage _ashealth_power_up _basedamage 0 0))
                  (:CastFailed
                    _))))
            (bind _returnvalue_3 (Game|Damage|ApplyDamage (.HitActor (Collision|BreakHitResult _outhit)) (Variables|Default|GetBaseDamage) 0 0))
            (bind _asvr_game_mode_test (Utilities|Casting|CastToVR_GameMode_Test (Game|GetGameMode))
              (:then
                _)
              (:CastFailed
                _))
            (Default|UpdateScore _asvr_game_mode_test _returnvalue_3)
            (Effects|SpawnEmitteratLocation "/Game/Move_Fodler/P_Explosion.P_Explosion" (.Location (Collision|BreakHitResult _outhit)) "0, 0, 0" "0.200000,0.200000,0.200000")
            (Effects|SpawnEmitteratLocation "/Game/VFX/Blood_VFX/Blood_Splat.Blood_Splat" (.Location (Collision|BreakHitResult _outhit)))
            (Audio|PlaySoundatLocation "/Game/Move_Fodler/Explosion02.Explosion02" (.Location (Collision|BreakHitResult _outhit)) "0, 0, 0" 0.3 1.0 0.0 0 0 0)
            (Utilities|FlowControl|Delay 0.5)
            (Variables|Default|SetCan%20Fire true)))))))

(event Input|ActionEvents|InputActionFireLeft
  (params (Key :type Key%20Structure))
  (bind _arrow (Variables|Default|GetArrow))
  (bind _arrow_muzzleflash (Variables|Default|GetArrow_Muzzleflash))
  (bind _basedamage (Variables|Default|GetBaseDamage))
  (bind _returnvalue (Transformation|GetWorldLocation _arrow))
  ;[1 1 1] Check if Firing in Correct Hand and fire line trace
  (:Pressed
    (if (Utilities|Enum|Equal(Enum) (Variables|/Game/VirtualRealityBP/Blueprints/BP_MotionController.BP_MotionController_C|GetHand (.AsBP%20Motion%20Controller (Utilities|Casting|CastToBP_MotionController (Components|GetOwner (Variables|Default|GetFirstHand))))) "Left")
      (if (Variables|Default|GetCan%20Fire)
        (if (<= (Variables|Default|GetAmmo) 0.0)
          (Audio|PlaySound2D "/Game/Designers/Audio/vo_reload_16.vo_reload_16" 1.0 1.0 0.0 0 0)
          (else
            (Variables|Default|SetAmmo (- (Variables|Default|GetAmmo) 1.0))
            (Variables|Default|SetCan%20Fire false)
            (Audio|PlaySound2D "/Game/Designers/Audio/Musket_Single_Shot_Close_03.Musket_Single_Shot_Close_03" 1.0 1.0 0.0 0 0)
            (bind _returnvalue_2 (Effects|SpawnEmitteratLocation "/Game/InfinityBladeEffects/Effects/FX_Monsters/FX_Monster_Chicken/P_ChickenMaster_MuzzleFlash_01.P_ChickenMaster_MuzzleFlash_01" (Transformation|GetWorldLocation _arrow_muzzleflash) (Transformation|GetWorldRotation _arrow_muzzleflash)))
            (Transformation|SetWorldScale3D _returnvalue_2 "0.200000,0.200000,0.200000")
            (bind _outhit (Collision|LineTraceByChannel _returnvalue (+ _returnvalue (* (Math|Vector|GetForwardVector _arrow) 5e+03)) "TraceTypeQuery2" false 0 "None"))
            (Utilities|FlowControl|Delay 0.35)
            (Variables|Default|SetCan%20Fire true)
            (bind _astime_power_up (Utilities|Casting|CastToTime_Power_Up (.HitActor (Collision|BreakHitResult _outhit)))
              (:then
                (Game|Damage|ApplyDamage _astime_power_up _basedamage 0 0))
              (:CastFailed
                (bind _ashealth_power_up (Utilities|Casting|CastToHealth_Power_Up (.HitActor (Collision|BreakHitResult _outhit)))
                  (:then
                    (Game|Damage|ApplyDamage _ashealth_power_up _basedamage 0 0))
                  (:CastFailed
                    _))))
            (bind _returnvalue_3 (Game|Damage|ApplyDamage (.HitActor (Collision|BreakHitResult _outhit)) (Variables|Default|GetBaseDamage) 0 0))
            (bind _asvr_game_mode_test (Utilities|Casting|CastToVR_GameMode_Test (Game|GetGameMode))
              (:then
                _)
              (:CastFailed
                _))
            (Default|UpdateScore _asvr_game_mode_test _returnvalue_3)
            (Effects|SpawnEmitteratLocation "/Game/Move_Fodler/P_Explosion.P_Explosion" (.Location (Collision|BreakHitResult _outhit)) "0, 0, 0" "0.200000,0.200000,0.200000")
            (Effects|SpawnEmitteratLocation "/Game/VFX/Blood_VFX/Blood_Splat.Blood_Splat" (.Location (Collision|BreakHitResult _outhit)))
            (Audio|PlaySoundatLocation "/Game/Move_Fodler/Explosion02.Explosion02" (.Location (Collision|BreakHitResult _outhit)) "0, 0, 0" 0.3 1.0 0.0 0 0 0)
            (Utilities|FlowControl|Delay 0.5)
            (Variables|Default|SetCan%20Fire true)))))))

(fn ConstructionScript)