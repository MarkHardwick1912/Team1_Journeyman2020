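; BP_Torch_Holding is a hand-held torch that BP_MotionController picks up and that can be lit from a BP_Torch.
; Pickup disables physics, attaches it to the given component and snaps the mesh to a fixed grip offset; Drop restores physics and detaches it.
; Overlapping a BP_Torch with its Sphere sets CanLight, and if still set after a short delay, the flame, audio and point light switch on.
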(event OnComponentBeginOverlap(Sphere)
  (params (OverlappedComponent :type Primitive%20Component%20Object%20Reference) (OtherActor :type Actor%20Object%20Reference) (OtherComp :type Primitive%20Component%20Object%20Reference) (OtherBodyIndex :type Integer) (bFromSweep :type Boolean) (SweepResult :type Hit%20Result%20Structure%20%28by%20ref%29))
  (Utilities|Casting|CastToBP_Torch OtherActor)
  (Variables|Default|SetCan%20Light true)
  (Utilities|FlowControl|Delay 2.0)
  (if (Variables|Default|GetCan%20Light)
    (Components|Activation|Activate (Variables|Default|GetAudio) false)
    (Rendering|SetVisibility (Variables|Default|GetPointLight) true false)))

(event OnComponentEndOverlap(Sphere)
  (params (OverlappedComponent :type Primitive%20Component%20Object%20Reference) (OtherActor :type Actor%20Object%20Reference) (OtherComp :type Primitive%20Component%20Object%20Reference) (OtherBodyIndex :type Integer))
  (Utilities|Casting|CastToBP_Torch OtherActor)
  (Variables|Default|SetCan%20Light false))

(event EventBeginPlay)

(event Collision|EventActorBeginOverlap
  (params (OtherActor :type Actor%20Object%20Reference)))

(event EventTick
  (params (DeltaSeconds :type Float%20%28single-precision%29)))

(event EventPickup
  (params (AttachTo :type Scene%20Component%20Object%20Reference))
  (Physics|SetSimulatePhysics (Variables|Debug|GetStaticMeshComponent) false)
  (Transformation|AttachComponentToComponent (VehicleSound|GetRootComponent) AttachTo "None" "KeepWorld" "KeepWorld" "KeepWorld" false)
  (Transformation|SetRelativeLocationAndRotation (Variables|Debug|GetStaticMeshComponent) "0,-2.315001,5.809070" "-10.000000, 0, 0" false true))

(event EventDrop
  (Physics|SetSimulatePhysics (Variables|Debug|GetStaticMeshComponent) true)
  (Transformation|DetachFromActor "KeepWorld" "KeepWorld" "KeepWorld"))

(fn ConstructionScript)