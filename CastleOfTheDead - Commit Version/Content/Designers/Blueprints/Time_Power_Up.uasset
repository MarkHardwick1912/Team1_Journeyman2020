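; Time power-up actor: a spinning hourglass that triggers slow motion when damage depletes its health.
; On depletion it hides the hourglass, disables its collision and plays a smash sound.
; After short delays and sound cues, it drops global time dilation to about 0.6, later restores near-normal speed, then destroys itself.
; Each FInterpTo runs only once, so speed changes are abrupt, and the delay runs in dilated time.
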(event EventTick
  (params (DeltaSeconds :type Float%20%28single-precision%29))
  (Transformation|AddActorLocalRotation (* (Math|Rotator|MakeRotator 0.0 0.0 (Variables|Default|GetRotationSpeed)) DeltaSeconds) false false))

(event Game|Damage|EventAnyDamage
  (params (Damage :type Float%20%28single-precision%29) (DamageType :type Damage%20Type%20Object%20Reference) (InstigatedBy :type Controller%20Object%20Reference) (DamageCauser :type Actor%20Object%20Reference))
  (bind _hourglass (Variables|Default|GetHourGlass))
  (bind _output_get (Variables|Default|SetEnemyHealth (- (Variables|Default|GetEnemyHealth) Damage)))
  (if (<= _output_get 0.0)
    (Collision|SetCollisionEnabled _hourglass "NoCollision")
    (Rendering|SetVisibility _hourglass false false)
    (Audio|PlaySound2D "/Game/Designers/Audio/Glass_Smash.Glass_Smash" 1.0 1.0 0.0 0 0)
    (Utilities|FlowControl|Delay 0.25)
    (Audio|PlaySound2D "/Game/Designers/Audio/Slo-Mo_Down.Slo-Mo_Down" 1.0 1.0 0.0 0 0)
    (Utilities|Time|SetGlobalTimeDilation (Math|Interpolation|FInterpTo 0.6 1.0 (stale EventTick DeltaSeconds) 1.0))
    (Utilities|FlowControl|Delay 1e+01)
    (Audio|PlaySound2D "/Game/Designers/Audio/Slo-Mo_Up.Slo-Mo_Up" 1.0 1.0 0.0 0 0)
    (Utilities|Time|SetGlobalTimeDilation (Math|Interpolation|FInterpTo 1.0 0.6 (stale EventTick DeltaSeconds) 1.0))
    (Actor|DestroyActor)))

(fn ConstructionScript)