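; Double door prop that swings two leaves open and closed, opening automatically when a VR motion controller overlaps its OpenCollision volume.
; A LerpTimer timeline interpolates each leaf's relative rotation between start and end rotators, playing to open and reversing to close.
; Open, Close and a FlipFlop toggle event drive the timeline.
; The construction script captures only the left leaf's start rotation from its placed transform.
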(event OnComponentBeginOverlap(OpenCollision)
  (params (OverlappedComponent :type Primitive%20Component%20Object%20Reference) (OtherActor :type Actor%20Object%20Reference) (OtherComp :type Primitive%20Component%20Object%20Reference) (OtherBodyIndex :type Integer) (bFromSweep :type Boolean) (SweepResult :type Hit%20Result%20Structure%20%28by%20ref%29))
  (Utilities|Casting|CastToBP_MotionController OtherActor)
  (CallFunction|Open))

(event Custom|Open
  (bind _alpha (Timeline|LerpTimer Play)
    (:Update
      (Utilities|FlowControl|Sequence
        (:then_0
          (Transformation|SetRelativeRotation (Variables|Default|GetDoor_Left) (Math|Rotator|Lerp(Rotator) (Variables|Default|GetStartRotation_left) (Variables|Default|GetEndRotation_left) _alpha) false false))
        (:then_1
          (Transformation|SetRelativeRotation (Variables|Default|GetDoor_Right) (Math|Rotator|Lerp(Rotator) (Variables|Default|GetStartRotation_right) (Variables|Default|GetEndRotation_right) _alpha) false false))))))

(event Custom|Close
  (bind _alpha (Timeline|LerpTimer Reverse)
    (:Update
      (Utilities|FlowControl|Sequence
        (:then_0
          (Transformation|SetRelativeRotation (Variables|Default|GetDoor_Left) (Math|Rotator|Lerp(Rotator) (Variables|Default|GetStartRotation_left) (Variables|Default|GetEndRotation_left) _alpha) false false))
        (:then_1
          (Transformation|SetRelativeRotation (Variables|Default|GetDoor_Right) (Math|Rotator|Lerp(Rotator) (Variables|Default|GetStartRotation_right) (Variables|Default|GetEndRotation_right) _alpha) false false))))))

(event Custom|Open/Close
  (Utilities|FlowControl|FlipFlop
    (:A
      (bind _alpha (Timeline|LerpTimer Play)
        (:Update
          (Utilities|FlowControl|Sequence
            (:then_0
              (Transformation|SetRelativeRotation (Variables|Default|GetDoor_Left) (Math|Rotator|Lerp(Rotator) (Variables|Default|GetStartRotation_left) (Variables|Default|GetEndRotation_left) _alpha) false false))
            (:then_1
              (Transformation|SetRelativeRotation (Variables|Default|GetDoor_Right) (Math|Rotator|Lerp(Rotator) (Variables|Default|GetStartRotation_right) (Variables|Default|GetEndRotation_right) _alpha) false false))))))
    (:B
      (Timeline|LerpTimer Reverse))))

(fn ConstructionScript
  (Variables|Default|SetStartRotation_left (Variables|/Script/Engine.SceneComponent|GetRelativeRotation (Variables|Default|GetDoor_Left))))