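; BP_Door_Single_Master is a single-leaf door prop that swings open and closed through Open, Close and a toggling Open/Close event.
; The construction script stores the door's starting relative rotation.
; The LerpTimer timeline then interpolates the door between that rotation and EndRotationLeft, playing forward to open and reversing to close, with a FlipFlop driving the toggle.
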(event Custom|Open
  (bind _alpha (Timeline|LerpTimer Play)
    (:Update
      (Utilities|FlowControl|Sequence
        (:then_0
          (Transformation|SetRelativeRotation (Variables|Default|GetDoor_Left) (Math|Rotator|Lerp(Rotator) (Variables|Default|GetStartRotation_left) (Variables|Default|GetEndRotation_left) _alpha) false false))))))

(event Custom|Close
  (bind _alpha (Timeline|LerpTimer Reverse)
    (:Update
      (Utilities|FlowControl|Sequence
        (:then_0
          (Transformation|SetRelativeRotation (Variables|Default|GetDoor_Left) (Math|Rotator|Lerp(Rotator) (Variables|Default|GetStartRotation_left) (Variables|Default|GetEndRotation_left) _alpha) false false))))))

(event Custom|Open/Close
  (Utilities|FlowControl|FlipFlop
    (:A
      (bind _alpha (Timeline|LerpTimer Play)
        (:Update
          (Utilities|FlowControl|Sequence
            (:then_0
              (Transformation|SetRelativeRotation (Variables|Default|GetDoor_Left) (Math|Rotator|Lerp(Rotator) (Variables|Default|GetStartRotation_left) (Variables|Default|GetEndRotation_left) _alpha) false false))))))
    (:B
      (Timeline|LerpTimer Reverse))))

(fn ConstructionScript
  (Variables|Default|SetStartRotation_left (Variables|/Script/Engine.SceneComponent|GetRelativeRotation (Variables|Default|GetDoor_Left))))