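; Trigger actor that spawns enemy AI when the MotionControllerPawn overlaps it, named for a heavy spawn in Level Two's final room.
; Overlap starts a looping half-second spawn timer, and the actor destroys itself after one second, limiting the burst to a couple of spawns.
; Each spawn indexes the Zombies and SpawnLoc arrays with random ranges fixed at zero, so only the first class and location are used.
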(event Custom|Spawner
  (AI|SpawnAIFromClass (Utilities|Array|Get(acopy) (Variables|Default|GetZombies) (Math|Random|RandomIntegerinRange 0 0)) 0 (Transformation|GetActorLocation (Utilities|Array|Get(acopy) (Variables|Default|GetSpawnLoc) (Math|Random|RandomIntegerinRange 0 0))) "0, 0, 0" true))

(event Collision|EventActorBeginOverlap
  (params (OtherActor :type Actor%20Object%20Reference))
  (Utilities|Casting|CastToMotionControllerPawn OtherActor)
  (Variables|Default|SetOverlapped true)
  (Utilities|Time|SetTimerbyEvent (delegate Custom|Spawner) 0.5 true)
  (Utilities|FlowControl|Delay 1.0)
  (Actor|DestroyActor))

(fn ConstructionScript)