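; VR crossbow pickup that also works as a sword when grabbed by its handle, which slides out a blade section.
; The holding hand's trigger fires a hitscan trace from the arrow, scaling damage on tagged enemies by hit bone.
; A second-hand overlap swaps in posed hand meshes and drives two-handed aiming on Tick, combining look-at between controllers with first-hand roll.
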(event OnComponentBeginOverlap(SecondHandTrigger)
  (params (OverlappedComponent :type Primitive%20Component%20Object%20Reference) (OtherActor :type Actor%20Object%20Reference) (OtherComp :type Primitive%20Component%20Object%20Reference) (OtherBodyIndex :type Integer) (bFromSweep :type Boolean) (SweepResult :type Hit%20Result%20Structure%20%28by%20ref%29))
  (bind _firsthand (Variables|Default|GetFirstHand))
  (bind _returnvalue (Components|GetOwner _firsthand))
  (bind _asbp_motion_controller (Utilities|Casting|CastToBP_MotionController _returnvalue))
  (bind _hand (Variables|/Game/VirtualRealityBP/Blueprints/BP_MotionController.BP_MotionController_C|GetHand _asbp_motion_controller))
  ;[1 1 1] Picking Up With Second Hand
  (if (not (Variables|Default|GetbGrabSwordHandle))
    (if (Variables|Default|GetbIsFirstHandAttached)
      (bind _asbp_motion_controller_2 (Utilities|Casting|CastToBP_MotionController OtherActor))
      (if (not (Actor|ActorHasTag (Variables|/Game/VirtualRealityBP/Blueprints/BP_MotionController.BP_MotionController_C|GetAttachedActor _asbp_motion_controller_2) "HeldObject"))
        (if (and (Utilities|Enum|Equal(Enum) (Variables|/Game/VirtualRealityBP/Blueprints/BP_MotionController.BP_MotionController_C|GetGripState _asbp_motion_controller_2) "NewEnumerator2") (!= (Variables|/Game/VirtualRealityBP/Blueprints/BP_MotionController.BP_MotionController_C|GetMotionController _asbp_motion_controller_2) _firsthand))
          (Variables|Default|SetbIsSecondHandTrackingActive true)
          (bind _output_get (Variables|Default|SetSecondHand (Variables|/Game/VirtualRealityBP/Blueprints/BP_MotionController.BP_MotionController_C|GetMotionController _asbp_motion_controller_2)))
          (Rendering|SetVisibility _output_get false false)
          (if (Utilities|Enum|Equal(Enum) _hand "Left")
            (Rendering|SetVisibility (Variables|Default|GetMannaquinHandRight%202) true false)
            (elif (Utilities|Enum|Equal(Enum) _hand "Right")
              (Rendering|SetVisibility (Variables|Default|GetMannequinLeft%20hand) true false))))))))

(event OnComponentEndOverlap(SecondHandTrigger)
  (params (OverlappedComponent :type Primitive%20Component%20Object%20Reference) (OtherActor :type Actor%20Object%20Reference) (OtherComp :type Primitive%20Component%20Object%20Reference) (OtherBodyIndex :type Integer))
  ;[1 1 1] Dropping Second hand
  (if (Variables|Default|GetbIsSecondHandTrackingActive)
    (Utilities|IsValid (Variables|Default|GetSecondHand)
      (:Is%20Valid
        (if (and (.bSuccess (Utilities|Casting|CastToBP_MotionController (Components|GetOwner (Variables|Default|GetSecondHand)))) (Utilities|Enum|NotEqual(Enum) (Variables|/Game/VirtualRealityBP/Blueprints/BP_MotionController.BP_MotionController_C|GetGripState (.AsBP%20Motion%20Controller (Utilities|Casting|CastToBP_MotionController (Components|GetOwner (Variables|Default|GetSecondHand))))) "NewEnumerator2"))
          (Variables|Default|SetbIsSecondHandTrackingActive false :!label _label)
          (Rendering|SetVisibility (Variables|/Game/VirtualRealityBP/Blueprints/BP_MotionController.BP_MotionController_C|GetHandMesh (stale OnComponentBeginOverlap(SecondHandTrigger) _asbp_motion_controller_2)) true false)
          (Variables|Default|SetSecondHand 0)
          (Transformation|SetRelativeRotation (Variables|Debug|GetStaticMeshComponent) (Variables|Default|GetOneHandRotation) false true)
          (Rendering|SetVisibility (Variables|Default|GetMannequinLeft%20hand) false false)))
      (:Is%20Not%20Valid
        (goto _label)))))

(event OnComponentBeginOverlap(SwordHandle)
  (params (OverlappedComponent :type Primitive%20Component%20Object%20Reference) (OtherActor :type Actor%20Object%20Reference) (OtherComp :type Primitive%20Component%20Object%20Reference) (OtherBodyIndex :type Integer) (bFromSweep :type Boolean) (SweepResult :type Hit%20Result%20Structure%20%28by%20ref%29))
  ;[1 1 1] Sword Handle
  (if (not (Variables|Default|GetbIsFirstHandAttached))
    (bind _asbp_motion_controller (Utilities|Casting|CastToBP_MotionController OtherActor))
    (Variables|Default|SetbGrabSwordHandle true)
    (if (Utilities|Enum|Equal(Enum) (Variables|/Game/VirtualRealityBP/Blueprints/BP_MotionController.BP_MotionController_C|GetGripState _asbp_motion_controller) "NewEnumerator2")
      (Physics|SetSimulatePhysics (Variables|Debug|GetStaticMeshComponent) false)
      (Transformation|AttachComponentToComponent (VehicleSound|GetRootComponent) (Variables|/Game/VirtualRealityBP/Blueprints/BP_MotionController.BP_MotionController_C|GetMotionController _asbp_motion_controller) "None" "SnapToTarget" "SnapToTarget" "KeepWorld" false)
      (Transformation|SetRelativeLocationAndRotation (Variables|Debug|GetStaticMeshComponent) "4.862000,-0.418000,30.716000" "0,-90.000000,-75.000000" false true)
      (Components|MoveComponentTo (Variables|Default|GetExtendable_Blade-Section) "0,10.000000, 0" "0, 0, 0" true false 0.1 false))))

(event OnComponentEndOverlap(SwordHandle)
  (params (OverlappedComponent :type Primitive%20Component%20Object%20Reference) (OtherActor :type Actor%20Object%20Reference) (OtherComp :type Primitive%20Component%20Object%20Reference) (OtherBodyIndex :type Integer))
  ;[1 1 1] Sword Handle
  (bind _asbp_motion_controller (Utilities|Casting|CastToBP_MotionController OtherActor))
  (Variables|Default|SetbGrabSwordHandle false)
  (if (Utilities|Enum|NotEqual(Enum) (Variables|/Game/VirtualRealityBP/Blueprints/BP_MotionController.BP_MotionController_C|GetGripState _asbp_motion_controller) "NewEnumerator2")
    (Physics|SetSimulatePhysics (Variables|Debug|GetStaticMeshComponent) true)
    (Transformation|DetachFromActor "KeepWorld" "KeepWorld" "KeepWorld")
    (Components|MoveComponentTo (Variables|Default|GetExtendable_Blade-Section) "0, 0, 0" "0, 0, 0" true false 0.1 false)))

(event EventPickup
  (params (AttachTo :type Scene%20Component%20Object%20Reference))
  ;[1 1 1] Picking Up Gun
  (if (not (Variables|Default|GetbGrabSwordHandle))
    (if (not (Variables|Default|GetbIsFirstHandAttached))
      (Physics|SetSimulatePhysics (Variables|Debug|GetStaticMeshComponent) false)
      (Transformation|AttachComponentToComponent (VehicleSound|GetRootComponent) AttachTo "None" "SnapToTarget" "SnapToTarget" "KeepWorld" false)
      (Transformation|SetRelativeLocationAndRotation (Variables|Debug|GetStaticMeshComponent) "18.507000,-0.269000,4.022000" (Variables|Default|GetOneHandRotation) false true)
      (Variables|Default|SetbIsFirstHandAttached true)
      (Variables|Default|SetbIsSecondHandTrackingActive false)
      (Variables|Default|SetFirstHand AttachTo)
      (Input|EnableInput (Game|GetPlayerController 0)))))

(event EventTick
  (params (DeltaSeconds :type Float%20%28single-precision%29))
  (bind _firsthand (Variables|Default|GetFirstHand))
  (bind _secondhand (Variables|Default|GetSecondHand))
  (bind _returnvalue (Transformation|GetWorldLocation _secondhand))
  (bind _returnvalue_2 (Transformation|GetWorldLocation _firsthand))
  (bind _returnvalue_3 (Math|Rotator|FindLookatRotation _returnvalue_2 _returnvalue))
  (bind (_roll _pitch _yaw) (Math|Rotator|BreakRotator _returnvalue_3))
  ;[1 1 1] 2 handed tracking
  (if (and (Variables|Default|GetbIsSecondHandTrackingActive) (Utilities|IsValid (Variables|Default|GetSecondHand)))
    (Transformation|SetWorldRotation (Variables|Debug|GetStaticMeshComponent) (Math|Rotator|CombineRotators (Variables|Default|GetOneHandRotation) (Math|Rotator|MakeRotator (.Roll (Math|Rotator|BreakRotator (Transformation|GetWorldRotation _firsthand))) _pitch _yaw)) false false)))

(event EventDrop
  ;[1 1 1] Dropping gun
  (Physics|SetSimulatePhysics (Variables|Debug|GetStaticMeshComponent) true)
  (Transformation|DetachFromActor "KeepWorld" "KeepWorld" "KeepWorld")
  (Variables|Default|SetbIsFirstHandAttached false)
  (Variables|Default|SetbIsSecondHandTrackingActive false)
  (Input|DisableInput (Game|GetPlayerController 0) 0))

(event Input|ActionEvents|InputActionFireRight
  (params (Key :type Key%20Structure))
  (bind _arrow (Variables|Default|GetArrow))
  (bind _returnvalue (Transformation|GetWorldLocation _arrow))
  ;[1 1 1] Check if Firing in Correct Hand and fire line trace
  (:Pressed
    (if (Utilities|Enum|Equal(Enum) (Variables|/Game/VirtualRealityBP/Blueprints/BP_MotionController.BP_MotionController_C|GetHand (.AsBP%20Motion%20Controller (Utilities|Casting|CastToBP_MotionController (Components|GetOwner (Variables|Default|GetFirstHand))))) "Right")
      (bind _outhit (Collision|LineTraceByChannel _returnvalue (+ _returnvalue (* (Math|Vector|GetForwardVector _arrow) 5e+03)) "TraceTypeQuery2" false 0 "ForDuration"))
      (if (Actor|ActorHasTag (.HitActor (Collision|BreakHitResult _outhit)) "Enemy")
        (switch name (.HitBoneName (Collision|BreakHitResult _outhit))
          (:Default
            (Game|Damage|ApplyDamage (.HitActor (Collision|BreakHitResult _outhit)) (Variables|Default|GetBaseDamage) 0 0)
            (Development|PrintString "chest"))
          (:head
            (Game|Damage|ApplyDamage (.HitActor (Collision|BreakHitResult _outhit)) (* (Variables|Default|GetBaseDamage) (Variables|Default|GetCritMult)) 0 0)
            (Development|PrintString "headshot"))
          (:lowerarm_l
            (Game|Damage|ApplyDamage (.HitActor (Collision|BreakHitResult _outhit)) (* (Variables|Default|GetBaseDamage) (Variables|Default|GetNonCritMult)) 0 0 :!label _label)
            (Development|PrintString "Arm"))
          (:upperarm_l
            (goto _label))
          (:lowerarm_r
            (goto _label))
          (:upperarm_r
            (goto _label))
          (:hand_l
            (goto _label))
          (:hand_r
            (goto _label)))
        (Effects|SpawnEmitteratLocation 0 (.Location (Collision|BreakHitResult _outhit)))
        (Audio|PlaySoundatLocation 0 "0, 0, 0" "0, 0, 0" 0.3 1.0 0.0 0 0 0)))))

(event Input|ActionEvents|InputActionFireLeft
  (params (Key :type Key%20Structure))
  (bind _arrow (Variables|Default|GetArrow))
  (bind _returnvalue (Transformation|GetWorldLocation _arrow))
  ;[1 1 1] Check if Firing in Correct Hand and fire line trace
  (:Pressed
    (if (Utilities|Enum|Equal(Enum) (Variables|/Game/VirtualRealityBP/Blueprints/BP_MotionController.BP_MotionController_C|GetHand (.AsBP%20Motion%20Controller (Utilities|Casting|CastToBP_MotionController (Components|GetOwner (Variables|Default|GetFirstHand))))) "Left")
      (bind _outhit (Collision|LineTraceByChannel _returnvalue (+ _returnvalue (* (Math|Vector|GetForwardVector _arrow) 5e+03)) "TraceTypeQuery2" false 0 "ForDuration"))
      (if (Actor|ActorHasTag (.HitActor (Collision|BreakHitResult _outhit)) "Enemy")
        (switch name (.HitBoneName (Collision|BreakHitResult _outhit))
          (:Default
            (Game|Damage|ApplyDamage (.HitActor (Collision|BreakHitResult _outhit)) (Variables|Default|GetBaseDamage) 0 0)
            (Development|PrintString "chest"))
          (:head
            (Game|Damage|ApplyDamage (.HitActor (Collision|BreakHitResult _outhit)) (* (Variables|Default|GetBaseDamage) (Variables|Default|GetCritMult)) 0 0)
            (Development|PrintString "headshot"))
          (:lowerarm_l
            (Game|Damage|ApplyDamage (.HitActor (Collision|BreakHitResult _outhit)) (* (Variables|Default|GetBaseDamage) (Variables|Default|GetNonCritMult)) 0 0 :!label _label)
            (Development|PrintString "Arm"))
          (:upperarm_l
            (goto _label))
          (:lowerarm_r
            (goto _label))
          (:upperarm_r
            (goto _label))
          (:hand_l
            (goto _label))
          (:hand_r
            (goto _label)))
        (Effects|SpawnEmitteratLocation 0 (.Location (Collision|BreakHitResult _outhit)))
        (Audio|PlaySoundatLocation 0 "0, 0, 0" "0, 0, 0" 0.3 1.0 0.0 0 0 0)))))

(fn ConstructionScript)