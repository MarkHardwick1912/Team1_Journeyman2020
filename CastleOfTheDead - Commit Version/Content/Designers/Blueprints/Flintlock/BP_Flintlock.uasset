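; BP_Flintlock is a VR flintlock pistol that motion controllers pick up, drop and fire.
; Pickup attaches it and swaps hand meshes; the matching hand's input spends ammo on a line trace, damaging enemies and power-ups, updating score and waiting out a fire delay.
; Melee overlaps damage enemies through a timeline-toggled cooldown gate, Tick swaps ammo and reload displays, and timelines drive dissolve effects.
; Bone-based critical damage logic exists but is disconnected.
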(event Custom|Disintegrate
  ;[1 1 1] Disintegration
  (bind _returnvalue (Rendering|Material|CreateDynamicMaterialInstance (Variables|Debug|GetStaticMeshComponent) 0 0 "None" :!class /Script/Engine.PrimitiveComponent))
  (bind _newtrack_0 (Timeline|Timeline_0 PlayFromStart)
    (:Update
      (Rendering|Material|SetScalarParameterValue _returnvalue "Amount" _newtrack_0 :!class /Script/Engine.MaterialInstanceDynamic))))

(event Custom|Reintegrate
  ;[1 1 1] Disintegration
  (bind _returnvalue (Rendering|Material|CreateDynamicMaterialInstance (Variables|Debug|GetStaticMeshComponent) 0 0 "None" :!class /Script/Engine.PrimitiveComponent))
  (bind _newtrack_0 (Timeline|Timeline_1 PlayFromStart)
    (:Update
      (Rendering|Material|SetScalarParameterValue _returnvalue "Amount" _newtrack_0 :!class /Script/Engine.MaterialInstanceDynamic))))

(event EventTick
  (params (DeltaSeconds :type Float%20%28single-precision%29))
  (if (<= (Variables|Default|GetAmmo) 0.0)
    (Rendering|SetVisibility (Variables|Default|GetReload) true false)
    (Rendering|SetVisibility (Variables|Default|GetAmmoCounter) false false)
    (else
      (Rendering|SetVisibility (Variables|Default|GetReload) false false)
      (Rendering|SetVisibility (Variables|Default|GetAmmoCounter) true false))))

(event EventPickup
  (params (AttachTo :type Scene%20Component%20Object%20Reference))
  ;[1 1 1] Picking Up Gun
  (Physics|SetSimulatePhysics (Variables|Debug|GetStaticMeshComponent) false)
  (Transformation|AttachComponentToComponent (VehicleSound|GetRootComponent) AttachTo "None" "SnapToTarget" "SnapToTarget" "KeepWorld" false)
  (Transformation|SetRelativeLocationAndRotation (Variables|Debug|GetStaticMeshComponent) "33.099998,-5.490000,9.060000" (Variables|Default|GetOneHandRotation) false true)
  (Variables|Default|SetFirstHand AttachTo)
  (Input|EnableInput (Game|GetPlayerController 0))
  (if (Utilities|Enum|Equal(Enum) (Variables|/Game/VirtualRealityBP/Blueprints/BP_MotionController.BP_MotionController_C|GetHand (.AsBP%20Motion%20Controller (Utilities|Casting|CastToBP_MotionController (Components|GetOwner (Variables|Default|GetFirstHand))))) "Right")
    (Rendering|SetVisibility (Variables|/Game/VirtualRealityBP/Blueprints/BP_MotionController.BP_MotionController_C|GetHandMesh (.AsBP%20Motion%20Controller (Utilities|Casting|CastToBP_MotionController (Components|GetOwner (Variables|Default|GetFirstHand))))) false false)
    (Rendering|SetVisibility (Variables|Default|GetMannequinHand_Right) true false)
    (elif (Utilities|Enum|Equal(Enum) (Variables|/Game/VirtualRealityBP/Blueprints/BP_MotionController.BP_MotionController_C|GetHand (.AsBP%20Motion%20Controller (Utilities|Casting|CastToBP_MotionController (Components|GetOwner (Variables|Default|GetFirstHand))))) "Left")
      (Rendering|SetVisibility (Variables|/Game/VirtualRealityBP/Blueprints/BP_MotionController.BP_MotionController_C|GetHandMesh (.AsBP%20Motion%20Controller (Utilities|Casting|CastToBP_MotionController (Components|GetOwner (Variables|Default|GetFirstHand))))) false false)
      (Rendering|SetVisibility (Variables|Default|GetMannequinHand_Left) true false))))

(event EventDrop
  ;[1 1 1] Dropping gun
  (Physics|SetSimulatePhysics (Variables|Debug|GetStaticMeshComponent) true)
  (Transformation|DetachFromActor "KeepWorld" "KeepWorld" "KeepWorld")
  (Input|DisableInput (Game|GetPlayerController 0) 0)
  (Rendering|SetVisibility (Variables|/Game/VirtualRealityBP/Blueprints/BP_MotionController.BP_MotionController_C|GetHandMesh (.AsBP%20Motion%20Controller (Utilities|Casting|CastToBP_MotionController (Components|GetOwner (Variables|Default|GetFirstHand))))) true false)
  (Rendering|SetVisibility (Variables|Default|GetMannequinHand_Left) false false))

(event Input|ActionEvents|InputActionFireRight
  (params (Key :type Key%20Structure))
  (bind _arrow (Variables|Default|GetArrow))
  (bind _returnvalue (Transformation|GetWorldLocation _arrow))
  ;[1 1 1] Check if Firing in Correct Hand and fire line trace
  (:Pressed
    (if (Utilities|Enum|Equal(Enum) (Variables|/Game/VirtualRealityBP/Blueprints/BP_MotionController.BP_MotionController_C|GetHand (.AsBP%20Motion%20Controller (Utilities|Casting|CastToBP_MotionController (Components|GetOwner (Variables|Default|GetFirstHand))))) "Right")
      (if (Variables|Default|GetCan%20Fire)
        (if (<= (Variables|Default|GetAmmo) 0.0)
          (Audio|PlaySound2D "/Game/Designers/Audio/vo_reload_16.vo_reload_16" 1.0 1.0 0.0 0 0)
          (else
            (Variables|Default|SetAmmo (- (Variables|Default|GetAmmo) 1.0))
            (Variables|Default|SetCan%20Fire false)
            (Audio|PlaySound2D "/Game/Designers/Audio/Flint_Quick_Mix_03.Flint_Quick_Mix_03" 1.0 1.0 0.0 0 0)
            (bind _outhit (Collision|LineTraceByChannel _returnvalue (+ _returnvalue (* (Math|Vector|GetForwardVector _arrow) 5e+03)) "TraceTypeQuery2" false 0 "None"))
            (bind _astime_power_up (Utilities|Casting|CastToTime_Power_Up (.HitActor (Collision|BreakHitResult _outhit)))
              (:then
                (Game|Damage|ApplyDamage _astime_power_up (Variables|Default|GetBaseDamage) 0 0))
              (:CastFailed
                _))
            (if (Actor|ActorHasTag (.HitActor (Collision|BreakHitResult _outhit)) "Enemy")
              (bind _returnvalue_2 (Game|Damage|ApplyDamage (.HitActor (Collision|BreakHitResult _outhit)) (Variables|Default|GetBaseDamage) 0 0))
              (bind _asvr_game_mode_test (Utilities|Casting|CastToVR_GameMode_Test (Game|GetGameMode)))
              (Default|UpdateScore _asvr_game_mode_test _returnvalue_2)
              (Effects|SpawnEmitteratLocation "/Game/Move_Fodler/P_Explosion.P_Explosion" (.Location (Collision|BreakHitResult _outhit)) "0, 0, 0" "0.500000,0.500000,0.500000")
              (Audio|PlaySoundatLocation "/Game/Move_Fodler/Explosion02.Explosion02" "0, 0, 0" "0, 0, 0" 0.3 1.0 0.0 0 0 0)
              (Utilities|FlowControl|Delay (Variables|Default|GetFire%20delay))
              (Variables|Default|SetCan%20Fire true)
              (else
                (Utilities|FlowControl|Delay (Variables|Default|GetFire%20delay))
                (Variables|Default|SetCan%20Fire true)
                (Effects|SpawnEmitteratLocation "/Game/Move_Fodler/P_Explosion.P_Explosion" "0, 0, 0" "0, 0, 0" "0.500000,0.500000,0.500000")))))))))

(event Input|ActionEvents|InputActionFireLeft
  (params (Key :type Key%20Structure))
  (bind _arrow (Variables|Default|GetArrow))
  (bind _returnvalue (Transformation|GetWorldLocation _arrow))
  ;[1 1 1] Check if Firing in Correct Hand and fire line trace
  (:Pressed
    (if (Utilities|Enum|Equal(Enum) (Variables|/Game/VirtualRealityBP/Blueprints/BP_MotionController.BP_MotionController_C|GetHand (.AsBP%20Motion%20Controller (Utilities|Casting|CastToBP_MotionController (Components|GetOwner (Variables|Default|GetFirstHand))))) "Left")
      (if (Variables|Default|GetCan%20Fire)
        (if (<= (Variables|Default|GetAmmo) 0.0)
          (Audio|PlaySound2D "/Game/Designers/Audio/vo_reload_16.vo_reload_16" 1.0 1.0 0.0 0 0)
          (else
            (Variables|Default|SetAmmo (- (Variables|Default|GetAmmo) 1.0))
            (Variables|Default|SetCan%20Fire false)
            (Audio|PlaySound2D "/Game/Designers/Audio/Flint_Quick_Mix_03.Flint_Quick_Mix_03" 1.0 1.0 0.0 0 0)
            (bind _outhit (Collision|LineTraceByChannel _returnvalue (+ _returnvalue (* (Math|Vector|GetForwardVector _arrow) 5e+03)) "TraceTypeQuery2" false 0 "None"))
            (bind _astime_power_up (Utilities|Casting|CastToTime_Power_Up (.HitActor (Collision|BreakHitResult _outhit)))
              (:then
                (Game|Damage|ApplyDamage _astime_power_up (Variables|Default|GetBaseDamage) 0 0))
              (:CastFailed
                _))
            (if (Actor|ActorHasTag (.HitActor (Collision|BreakHitResult _outhit)) "Enemy")
              (bind _returnvalue_2 (Game|Damage|ApplyDamage (.HitActor (Collision|BreakHitResult _outhit)) (Variables|Default|GetBaseDamage) 0 0))
              (bind _asvr_game_mode_test (Utilities|Casting|CastToVR_GameMode_Test (Game|GetGameMode)))
              (Default|UpdateScore _asvr_game_mode_test _returnvalue_2)
              (Effects|SpawnEmitteratLocation "/Game/Move_Fodler/P_Explosion.P_Explosion" (.Location (Collision|BreakHitResult _outhit)) "0, 0, 0" "0.500000,0.500000,0.500000")
              (Audio|PlaySoundatLocation "/Game/Move_Fodler/Explosion02.Explosion02" "0, 0, 0" "0, 0, 0" 0.3 1.0 0.0 0 0 0)
              (Utilities|FlowControl|Delay (Variables|Default|GetFire%20delay))
              (Variables|Default|SetCan%20Fire true)
              (else
                (Utilities|FlowControl|Delay (Variables|Default|GetFire%20delay))
                (Variables|Default|SetCan%20Fire true)
                (Effects|SpawnEmitteratLocation "/Game/Move_Fodler/P_Explosion.P_Explosion" "0, 0, 0" "0, 0, 0" "0.500000,0.500000,0.500000")))))))))

(event OnComponentBeginOverlap(Melee_Collision)
  (params (OverlappedComponent :type Primitive%20Component%20Object%20Reference) (OtherActor :type Actor%20Object%20Reference) (OtherComp :type Primitive%20Component%20Object%20Reference) (OtherBodyIndex :type Integer) (bFromSweep :type Boolean) (SweepResult :type Hit%20Result%20Structure%20%28by%20ref%29))
  ;[1 1 1] Collision target and damage application
  (if (Actor|ActorHasTag OtherActor "Enemy")
    (Utilities|FlowControl|Gate false
      (:Exit
        (Game|Damage|ApplyDamage OtherActor (Variables|Default|GetMelee_Damage) 0 0)
        ;[1 1 1] Melee cooldown handle
        (CallFunction|MeleeToggle)
        (Components|Timeline|SetPlayRate (Variables|Default|GetCooldown_Timeline) (/ 1.0 (Variables|Default|GetMelee_Cooldown)))
        (bind _alpha (Timeline|Cooldown_Timeline PlayFromStart)
          (:Update
            (if (== (Math|Float|Lerp 0.0 1.0 _alpha) 1.0)
              (CallFunction|MeleeToggle))))))))

(event Custom|Melee_Toggle
  ;[1 1 1] Collision target and damage application
  (Utilities|FlowControl|Gate false) ; enters at Toggle
)

(fn ConstructionScript)