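; VR_GameMode_Test is a game mode Blueprint that creates the score display and keeps a running score based on damage.
; On BeginPlay it creates a ScoreWidget for the first player controller and adds it to the viewport.
; UpdateScore multiplies applied damage by PPD, adds it to CurrentScore and stores the rounded total as a float.
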(event EventBeginPlay
  (bind _returnvalue (UserInterface|CreateWidget "/Game/Designers/Blueprints/ScoreWidget.ScoreWidget_C" (Game|GetPlayerController 0)))
  (UserInterface|Viewport|AddtoViewport _returnvalue 0))

(fn ConstructionScript)

(fn UpdateScore
  (params (DamageApplied :type Float%20%28single-precision%29))
  (Variables|Default|SetCurrentScore (Math|Conversions|ToFloat(Integer) (Math|Float|Round (+ (* DamageApplied (Variables|Default|GetPPD)) (Variables|Default|GetCurrentScore))))))