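; Shootable health power-up actor that spins an hourglass at a set rotation speed every tick.
; Damage drains its health; at zero it hides both hourglass meshes, disables their collision and plays a glass smash.
; After a short delay it increments the MotionControllerPawn's current health and destroys itself.
; An unconnected chain of slow-motion sound and time-dilation nodes remains in the graph but never runs.
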(event EventTick
  (params (DeltaSeconds :type Float%20%28single-precision%29))
  (Transformation|AddActorLocalRotation (* (Math|Rotator|MakeRotator 0.0 0.0 (Variables|Default|GetRotationSpeed)) DeltaSeconds) false false))

(event Game|Damage|EventAnyDamage
  (params (Damage :type Float%20%28single-precision%29) (DamageType :type Damage%20Type%20Object%20Reference) (InstigatedBy :type Controller%20Object%20Reference) (DamageCauser :type Actor%20Object%20Reference))
  (bind _hourglass (Variables|Default|GetHourGlass))
  (bind _output_get (Variables|Default|SetEnemyHealth (- (Variables|Default|GetEnemyHealth) Damage)))
  (if (<= _output_get 0.0)
    (Collision|SetCollisionEnabled _hourglass "NoCollision")
    (Rendering|SetVisibility _hourglass false false)
    (Audio|PlaySound2D "/Game/Designers/Audio/Glass_Smash.Glass_Smash" 1.0 1.0 0.0 0 0)
    (Utilities|FlowControl|Delay 0.25)
    (bind _asmotion_controller_pawn (Utilities|Casting|CastToMotionControllerPawn (Game|Player|GetPlayerPawn 0)))
    (Math|Float|IncrementFloat (Variables|/Game/VirtualRealityBP/Blueprints/MotionControllerPawn.MotionControllerPawn_C|GetCurrentHealth _asmotion_controller_pawn)
      (:%20%20
        (Actor|DestroyActor)))))

(fn ConstructionScript)